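; BP_CryStal is a crystal with health that monsters attack, and losing all crystals is meant to end the game.
; A BP_Monster overlapping its Box gets CryStalDie called and costs the crystal a fixed, clamped amount of health, shown on its WBP_CryStalHealth widget.
; At zero health it flags itself destroyed, and JudgeIsDie ANDs that flag across all crystals to trigger GameOver(false) on WBP_HUD.
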(event `self.ReceiveBeginPlay`
  (set `self.当前生命值` (`self.总生命数`))
  (bind _aswbp_cry_stal_health (cast `/Game/BP/WBP/WBP_CryStalHealth` (`WidgetComponent.GetWidget` (`self.Widget`))))
  (set `self.HealthWidget` _aswbp_cry_stal_health))

(event `self.Box.OnComponentBeginOverlap`
  (params (OverlappedComponent :type "PrimitiveComponent Object Reference") (OtherActor :type "Actor Object Reference") (OtherComp :type "PrimitiveComponent Object Reference") (OtherBodyIndex :type Integer) (bFromSweep :type Boolean) (SweepResult :type "HitResult Structure (by ref)"))
  (bind _healthwidget (`self.HealthWidget`))
  (bind _asbp_monster (cast `/Game/BP/BP_Monster` OtherActor))
  (`/Game/BP/BP_Monster.CryStalDie` _asbp_monster)
  (bind _output_get (set `self.当前生命值` (`KismetMathLibrary.Clamp` (- (`self.当前生命值`) (`self.攻击扣减生命值`)) 0 (`self.总生命数`))))
  (`/Game/EditorBlueprintResources/StandardMacros.IsValid` _healthwidget
    (:`Is Valid`
      (`/Game/BP/WBP/WBP_CryStalHealth.SetHealth` _healthwidget (`self.总生命数`) (`self.当前生命值`))
      (bind _output_get_2 (set `self.是否被击破` (<= _output_get 0)))
      (if _output_get_2
        (bind _newparam (`self.JudgeIsDie`))
        (if _newparam
          (bind _foundwidgets (`WidgetBlueprintLibrary.GetAllWidgetsOfClass` "/Game/BP/WBP/WBP_HUD.WBP_HUD_C"))
          (`/Game/BP/WBP/WBP_HUD.GameOver` (`|GetArrayItem` _foundwidgets) false))))))

(event `self.Box.OnComponentEndOverlap`
  (params (OverlappedComponent :type "PrimitiveComponent Object Reference") (OtherActor :type "Actor Object Reference") (OtherComp :type "PrimitiveComponent Object Reference") (OtherBodyIndex :type Integer)))

(fn `JudgeIsDie`
  (returns (NewParam :type Boolean))
  (locals (lob_bool :type Boolean :default true))
  (bind _outactors (`GameplayStatics.GetAllActorsOfClass` "BP_CryStal_C"))
  (bind _array_element (`/Game/EditorBlueprintResources/StandardMacros.ForEachLoop` _outactors)
    (:`LoopBody`
      (set `local.lob_bool` (and (`/Game/BP/BP_CryStal.是否被击破` _array_element) (`local.lob_bool`))))
    (:`Completed`
      (return (`local.lob_bool`)))))

(fn `UserConstructionScript`)