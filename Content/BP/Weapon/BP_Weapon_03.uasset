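; BP_Weapon_03 is a child weapon Blueprint that deals area damage to monsters around itself.
; On BeginPlay it spawns a scaled-up Warrior spin particle at its location and stores it in Lizi.
; The WWgongi attack event runs a zero-length multi sphere trace on Visibility and calls WWshoushang on hit BP_Monster actors, stopping at a failed cast.
; PlayAnim extends the parent by playing a one-shot gun fire animation.
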(event `self.ReceiveBeginPlay`
  (`parent.ReceiveBeginPlay`)
  (bind _returnvalue (`GameplayStatics.SpawnEmitterAtLocation` "/Game/RPGEffects/Particles/P_Warrior_Spin.P_Warrior_Spin" (`self.K2_GetActorLocation`) (struct) (3.0 3.0 2.0)))
  (set `self.lizi` _returnvalue))

(event `self.WWgongi`
  (bind _returnvalue (`self.K2_GetActorLocation`))
  (bind _outhits (`KismetSystemLibrary.SphereTraceMulti` _returnvalue _returnvalue 650.0 "TraceTypeQuery1"))
  (bind _array_element (`/Game/EditorBlueprintResources/StandardMacros.ForEachLoop` _outhits)
    (:`LoopBody`
      (bind _asbp_monster (cast `/Game/BP/BP_Monster` (`.HitActor` (`GameplayStatics.BreakHitResult` _array_element))))
      (`/Game/BP/BP_Monster.WWshoushang` _asbp_monster 4))))

(fn `PlayAnim`
  (`parent.PlayAnim`)
  (`SkeletalMeshComponent.PlayAnimation` (`self.SkeletalMesh`) "/Game/CSC/Animations/Anim_CSC_Gun6_Fire.Anim_CSC_Gun6_Fire" false))

(fn `UserConstructionScript`
  (`parent.UserConstructionScript`))