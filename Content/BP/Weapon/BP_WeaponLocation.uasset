(event `SpawnFiled`
  (set `self.isClick` false))

(event `SpawnWeapon`
  (params (InData :type "/Game/BP/Data/DS_Weapon Structure"))
  (bind ((`Id_2_B497C63B4A0B9050F859CB984797D97F` _id) (`Class_8_1264049A40E6D486F0AFE1A3FE640349` _class)) (break `/Game/BP/Data/DS_Weapon` InData))
  (bind _weapon (`self.Weapon`))
  (set `self.isClick` false)
  (set `self.Id` _id)
  (if (`self.isBuilding`)
    (`/Game/EditorBlueprintResources/StandardMacros.IsValid` _weapon
      (:`Is Valid`
        (`self.K2_DestroyActor` _weapon))
      (:`Is Not Valid`
        _)))
  (bind _returnvalue (`|SpawnActorFromClass` _class (`KismetMathLibrary.MakeTransform` (`SceneComponent.K2_GetComponentLocation` (`self.Scene`))) "Undefined" "MultiplyWithRoot" null null))
  (set `self.Weapon` _returnvalue)
  (set `/Game/BP/Weapon/BP_Weapon.Loaction` self _returnvalue)
  (set `self.isBuilding` true))

(event `self.Plane.OnClicked`
  (params (TouchedComponent :type "PrimitiveComponent Object Reference") (ButtonPressed :type "Key Structure")))

(event `self.Box.OnClicked`
  (params (TouchedComponent :type "PrimitiveComponent Object Reference") (ButtonPressed :type "Key Structure"))
  (bind `_as游戏实例` (cast `/Game/BP/游戏实例` (`GameplayStatics.GetGameInstance`) :!pure true))
  (bind _is_show (`/Game/BP/游戏实例.is show` `_as游戏实例`))
  (if (not (`self.isClick`))
    (bind _outactors (`GameplayStatics.GetAllActorsOfClass` "BP_WeaponLocation_C"))
    (bind _array_element (`/Game/EditorBlueprintResources/StandardMacros.ForEachLoop` _outactors)
      (:`LoopBody`
        (set `/Game/BP/Weapon/BP_WeaponLocation.isClick` false _array_element))
      (:`Completed`
        (set `self.isClick` true)
        (if (== (`self.Id`) -1)
          (`/Game/EditorBlueprintResources/StandardMacros.IsValid` (`self.Widget`) :!label _label
            (:`Is Valid`
              (if (`self.isBuilding`)
                (if _is_show
                  (set `/Game/BP/游戏实例.is show` false `_as游戏实例`)
                  (`/Game/BP/WBP/WBP_Main.WeaponUp` (`self.Widget`) (`self.Id`) self))
                (elif _is_show
                  (set `/Game/BP/游戏实例.is show` false `_as游戏实例`)
                  (`/Game/BP/WBP/WBP_Main.WeaponCreate` (`self.Widget`) self)))))
          (else
            (bind _outrownames (`DataTableFunctionLibrary.GetDataTableRowNames` "/Game/BP/Data/DT_Weapon.DT_Weapon"))
            (bind _array_element_2 (`/Game/EditorBlueprintResources/StandardMacros.ForEachLoop` _outrownames)
              (:`LoopBody`
                (bind _returnvalue (`|GetDataTableRow` "/Game/BP/Data/DT_Weapon.DT_Weapon" _array_element_2)
                  (:`then`
                    (bind ((`Id_2_B497C63B4A0B9050F859CB984797D97F` _id) (`UpId_16_18BFFE0246E3F91AD49246A6F3FE21F9` _upid)) (break `/Game/BP/Data/DS_Weapon` _returnvalue))
                    (if (== _id (`self.Id`))
                      (if (== _upid -1)
                        (set `self.isClick` false)
                        (else
                          (goto _label))))))))))))))

(event `SetPlayerLocation`
  (bind _returnvalue (`GameplayStatics.GetPlayerController` 0))
  (bind _arrow (`self.Arrow`))
  (bind _returnvalue_2 (`SceneComponent.K2_GetComponentRotation` _arrow))
  (`self.K2_SetActorLocationAndRotation` (`Controller.K2_GetPawn` _returnvalue) (`SceneComponent.K2_GetComponentLocation` _arrow) _returnvalue_2 false false)
  (`Controller.SetControlRotation` _returnvalue _returnvalue_2))

(event `ColorWeapon`
  (set `self.isClick` false))

(event `WWChongzhi`
  (bind _weapon (`self.Weapon`))
  (`/Game/EditorBlueprintResources/StandardMacros.IsValid` _weapon
    (:`Is Valid`
      (bind _asbp_player (cast `/Game/BP/Player/BP_Player` (`GameplayStatics.GetPlayerCharacter` 0)))
      (set `/Game/BP/Player/BP_Player.jingBi` (+ (`/Game/BP/Player/BP_Player.jingBi` _asbp_player) (* (`self.Id`) 7)) _asbp_player)
      (bind _asbp_weapon_03 (cast `/Game/BP/Weapon/BP_Weapon_03` _weapon)
        (:`then`
          (`ActorComponent.K2_DestroyComponent` (`/Game/BP/Weapon/BP_Weapon_03.lizi` _asbp_weapon_03)))
        (:`CastFailed`
          _))
      (`self.K2_DestroyActor` _weapon)
      (set `self.isBuilding` false)
      (set `self.Id` -1))))

(event `self.ReceiveBeginPlay`
  (`KismetSystemLibrary.Delay` 2.0)
  (bind _foundwidgets (`WidgetBlueprintLibrary.GetAllWidgetsOfClass` "/Game/BP/WBP/WBP_HUD.WBP_HUD_C"))
  (set `self.Widget` (`/Game/BP/WBP/WBP_HUD.WBP_Main` (`|GetArrayItem` _foundwidgets))))

(fn `UserConstructionScript`)