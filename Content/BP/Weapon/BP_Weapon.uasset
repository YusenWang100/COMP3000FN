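; Auto-firing weapon actor that targets BP_Monster actors entering its range.
; Cylinder overlaps maintain the monster list, and the construction script sizes the Sphere and Cylinder from Radius.
; BeginPlay caches scene components tagged "Bullet" as muzzles and starts a looping fire timer.
; Each tick of that timer turns the actor toward the first listed monster, spawns BP_Bullet at every muzzle, and calls an empty PlayAnim.
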(event `self.ReceiveBeginPlay`
  (`KismetSystemLibrary.PrintString` "Hello")
  (bind _array_element (`/Game/EditorBlueprintResources/StandardMacros.ForEachLoop` (`self.K2_GetComponentsByClass` "/Script/Engine.SceneComponent"))
    (:`LoopBody`
      (if (`KismetArrayLibrary.Array_Contains` (`ActorComponent.ComponentTags` _array_element) "Bullet")
        (`KismetArrayLibrary.Array_Add` (`self.NewVar`) _array_element)))
    (:`Completed`
      (`KismetSystemLibrary.K2_SetTimerDelegate` (delegate `SpawnBullet`) (`self.Time`) true))))

(event `SpawnBullet`
  (`self.WWgongi`))

(event `WWgongi`
  (bind _output (`|GetArrayItem` (`self.Monsters`)))
  (`/Game/EditorBlueprintResources/StandardMacros.IsValid` _output
    (:`Is Valid`
      (`self.K2_SetActorRotation` (`KismetMathLibrary.FindLookAtRotation` (`self.K2_GetActorLocation`) (`self.K2_GetActorLocation` _output)))
      (bind _array_element (`/Game/EditorBlueprintResources/StandardMacros.ForEachLoop` (`self.NewVar`))
        (:`LoopBody`
          (`|SpawnActorFromClass` "/Game/BP/Weapon/BP_Bullet.BP_Bullet_C" (`KismetMathLibrary.MakeTransform` (`SceneComponent.K2_GetComponentLocation` _array_element) (`SceneComponent.K2_GetComponentRotation` _array_element)) "Undefined" "MultiplyWithRoot" null 1 null))
        (:`Completed`
          (`self.PlayAnim`))))))

(event `self.Cylinder.OnComponentBeginOverlap`
  (params (OverlappedComponent :type "PrimitiveComponent Object Reference") (OtherActor :type "Actor Object Reference") (OtherComp :type "PrimitiveComponent Object Reference") (OtherBodyIndex :type Integer) (bFromSweep :type Boolean) (SweepResult :type "HitResult Structure (by ref)"))
  (bind _asbp_monster (cast `/Game/BP/BP_Monster` OtherActor))
  (`KismetArrayLibrary.Array_Add` (`self.Monsters`) _asbp_monster))

(event `self.Cylinder.OnComponentEndOverlap`
  (params (OverlappedComponent :type "PrimitiveComponent Object Reference") (OtherActor :type "Actor Object Reference") (OtherComp :type "PrimitiveComponent Object Reference") (OtherBodyIndex :type Integer))
  (bind _asbp_monster (cast `/Game/BP/BP_Monster` OtherActor))
  (`KismetArrayLibrary.Array_RemoveItem` (`self.Monsters`) _asbp_monster))

(event `WWchanchu`)

(event `self.Sphere.OnComponentEndOverlap`
  (params (OverlappedComponent :type "PrimitiveComponent Object Reference") (OtherActor :type "Actor Object Reference") (OtherComp :type "PrimitiveComponent Object Reference") (OtherBodyIndex :type Integer)))

(fn `PlayAnim`)

(fn `UserConstructionScript`
  (`SphereComponent.SetSphereRadius` (`self.Sphere`) (`self.Radius`) true)
  (`SceneComponent.SetRelativeScale3D` (`self.Cylinder`) (`KismetMathLibrary.Conv_DoubleToVector` (* (/ (`self.Radius`) 100.0) 2.0))))