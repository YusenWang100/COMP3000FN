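; BP_Monster is an enemy that travels along an attack-route spline belonging to a crystal and dies to damage.
; At BeginPlay it scales health from game instance values and picks a random route from a random unbroken BP_CryStal.
; Tick advances it along the spline by a fixed per-frame step.
; Bullet overlaps or WWshoushang reduce health; at zero it rewards the player and destroys itself, while CryStalDie destroys it without reward.
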(event `self.ReceiveBeginPlay`
  (bind _outitem (`KismetArrayLibrary.Array_Random` (`self.Array Element`)))
  (bind `_as游戏实例` (cast `/Game/BP/游戏实例` (`GameplayStatics.GetGameInstance`) :!pure true))
  (set `self.CurrentHealth` (* (`/Game/BP/游戏实例.敌人血量` `_as游戏实例`) (`/Game/BP/游戏实例.11` `_as游戏实例`)))
  (bind _outactors (`GameplayStatics.GetAllActorsOfClass` "/Game/BP/BP_CryStal.BP_CryStal_C"))
  (bind _array_element (`/Game/EditorBlueprintResources/StandardMacros.ForEachLoop` _outactors)
    (:`LoopBody`
      (if (not (`/Game/BP/BP_CryStal.是否被击破` _array_element))
        (`KismetArrayLibrary.Array_Add` (`self.Array Element`) _array_element)))
    (:`Completed`
      (`/Game/EditorBlueprintResources/StandardMacros.IsValid` _outitem
        (:`Is Valid`
          (set `self.NewVar` (`KismetArrayLibrary.Array_Random` (`/Game/BP/BP_CryStal.攻击路线` _outitem))))))))

(event `self.ReceiveTick`
  (params (DeltaSeconds :type "Float (single-precision)"))
  (bind _newvar (`self.NewVar`))
  (bind _distance (`self.Distance`))
  (bind _returnvalue (+ (`self.Distance`) (`self.Speed`)))
  (bind _spline (`/Game/BP/BP_Path.Spline` _newvar))
  (`|ExecutionSequence`
    (:`then_0`
      (`/Game/EditorBlueprintResources/StandardMacros.IsValid` _newvar
        (:`Is Valid`
          (if (not (> _returnvalue (`SplineComponent.GetSplineLength` _spline)))
            (set `self.Distance` _returnvalue)
            (`self.K2_SetActorLocationAndRotation` (`SplineComponent.GetLocationAtDistanceAlongSpline` _spline _distance "World") (`SplineComponent.GetRotationAtDistanceAlongSpline` _spline _distance "World"))))))))

(event `self.Cube.OnComponentBeginOverlap`
  (params (OverlappedComponent :type "PrimitiveComponent Object Reference") (OtherActor :type "Actor Object Reference") (OtherComp :type "PrimitiveComponent Object Reference") (OtherBodyIndex :type Integer) (bFromSweep :type Boolean) (SweepResult :type "HitResult Structure (by ref)"))
  (bind `_as游戏实例` (cast `/Game/BP/游戏实例` (`GameplayStatics.GetGameInstance`) :!pure true))
  (bind _asbp_bullet (cast `/Game/BP/Weapon/BP_Bullet` OtherActor))
  (set `self.CurrentHealth` (`KismetMathLibrary.Clamp` (- (`self.CurrentHealth`) (`/Game/BP/Weapon/BP_Bullet.HitNumber` _asbp_bullet)) 0 (* (`/Game/BP/游戏实例.敌人血量` `_as游戏实例`) (`/Game/BP/游戏实例.11` `_as游戏实例`))))
  (`/Game/EditorBlueprintResources/StandardMacros.IsValid` _asbp_bullet
    (:`Is Valid`
      (`self.K2_DestroyActor` _asbp_bullet))
    (:`Is Not Valid`
      _))
  (if (== (`self.CurrentHealth`) 0) :!label _label
    (`KismetSystemLibrary.DelayUntilNextTick`)
    (`self.BulletDie`)))

(event `WWshoushang`
  (params (B :type Integer))
  (bind `_as游戏实例` (cast `/Game/BP/游戏实例` (`GameplayStatics.GetGameInstance`) :!pure true))
  (set `self.CurrentHealth` (`KismetMathLibrary.Clamp` (- (`self.CurrentHealth`) B) 0 (* (`/Game/BP/游戏实例.敌人血量` `_as游戏实例`) (`/Game/BP/游戏实例.11` `_as游戏实例`))))
  (goto _label))

(event `BulletDie`
  (`|ExecutionSequence`
    (:`then_0`
      (bind _asbp_player (cast `/Game/BP/Player/BP_Player` (`Controller.K2_GetPawn` (`GameplayStatics.GetPlayerController` 0))))
      (`/Game/BP/Player/BP_Player.SetData` _asbp_player (`self.number`) (`/Game/BP/游戏实例.金币` (cast `/Game/BP/游戏实例` (`GameplayStatics.GetGameInstance`) :!pure true))))
    (:`then_1`
      (`self.K2_DestroyActor`))))

(event `CryStalDie`
  (`self.K2_DestroyActor`))

(fn `UserConstructionScript`)