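; BP_Spawn is a monster spawner actor that creates waves of monsters and reports to the HUD when a wave is cleared.
; SpawnMustor loops over the requested count at randomly offset positions, spawning either double-scale BP_Monster_Child instantly or BP_Monster after a delay each.
; Spawns are tracked in an array with destroy bindings, and MonsterDestory counts down to notify the WBP_HUD main widget cached at BeginPlay.
; The timer-driven SS spawn path is unconnected.
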(event `SpawnMustor`
  (params (Number :type Integer) (Time :type "Float (double-precision)") (Condition :type Boolean))
  (bind _monsters (`self.Monsters`))
  (bind _returnvalue (`KismetMathLibrary.RandomFloatInRange` 0.0 (`self.Random`)))
  (bind _returnvalue_2 (+ (`self.K2_GetActorLocation`) (* (`self.GetActorRightVector`) _returnvalue) (* (`self.GetActorForwardVector`) _returnvalue) (* (`self.GetActorUpVector`) 90.0)))
  (bind _output_get (set `self.Number` Number))
  (set `self.loc_Number` _output_get)
  (if (not (<= (`self.loc_Number`) 0)) :!label _label
    (if Condition
      (bind _returnvalue_3 (`|SpawnActorFromClass` "/Game/BP/BP_Monster_Child.BP_Monster_Child_C" (`KismetMathLibrary.MakeTransform` _returnvalue_2 (struct) (2.0 2.0 2.0)) "AdjustIfPossibleButAlwaysSpawn" "MultiplyWithRoot" null null))
      (`KismetArrayLibrary.Array_Add` _monsters _returnvalue_3)
      (add `self.OnDestroyed` _returnvalue_3 (`|CreateDelegate` :!event `MonsterDestory`))
      (else
        (`KismetSystemLibrary.Delay` Time)
        (bind _returnvalue_4 (`|SpawnActorFromClass` "/Game/BP/BP_Monster.BP_Monster_C" (`KismetMathLibrary.MakeTransform` _returnvalue_2) "Undefined" "MultiplyWithRoot" null null))
        (`KismetArrayLibrary.Array_Add` _monsters _returnvalue_4)
        (add `self.OnDestroyed` _returnvalue_4 (`|CreateDelegate` :!event `MonsterDestory`))))
    (`/Game/EditorBlueprintResources/StandardMacros.DecrementInt` (`self.loc_Number`)
      (:`  `
        (goto _label)))))

(event `self.ReceiveBeginPlay`
  (`KismetSystemLibrary.Delay` 0.2)
  (bind _foundwidgets (`WidgetBlueprintLibrary.GetAllWidgetsOfClass` "/Game/BP/WBP/WBP_HUD.WBP_HUD_C"))
  (set `self.Widget` (`/Game/BP/WBP/WBP_HUD.WBP_Main` (`|GetArrayItem` _foundwidgets))))

(event `SS`
  (bind _returnvalue (`KismetMathLibrary.RandomFloatInRange` 0.0 (`self.Random`)))
  (`|SpawnActorFromClass` "/Game/BP/BP_Monster.BP_Monster_C" (`KismetMathLibrary.MakeTransform` (+ (`self.K2_GetActorLocation`) (* (`self.GetActorRightVector`) _returnvalue) (* (`self.GetActorForwardVector`) _returnvalue) (* (`self.GetActorUpVector`) 90.0))) "Undefined" "MultiplyWithRoot" null null))

(event `MonsterDestory` :!signature `self.OnDestroyed`
  (params (DestroyedActor :type "Actor Object Reference"))
  (bind _widget (`self.Widget`))
  (bind _result (`/Game/EditorBlueprintResources/StandardMacros.DecrementInt` (`self.Number`))
    (:`  `
      (if (== _result 0)
        (`/Game/EditorBlueprintResources/StandardMacros.IsValid` _widget
          (:`Is Valid`
            (`/Game/BP/WBP/WBP_Main.MonsterDestoryEvent` _widget)))))))

(fn `UserConstructionScript`)